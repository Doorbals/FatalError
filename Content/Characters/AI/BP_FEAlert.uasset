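; BP_FEAlert is an alert actor that switches on a linked alert light when an alert is pushed.
; Its PushAlert event calls the parent behaviour, then enables the AlertLight actor's tick and raises both of its spotlights to high intensity.
; After a fixed delay of several seconds, it turns both spotlights off and disables that actor's tick again.
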(event EventBeginPlay)

(event Collision|EventActorBeginOverlap
  (params (OtherActor :type Actor%20Object%20Reference)))

(event EventPushAlert
  (bind _alertlight (Variables|Default|GetAlertLight))
  (bind _spotlight (Variables|/Game/Characters/AI/BP_AlertLight.BP_AlertLight_C|GetSpotLight _alertlight))
  (bind _spotlight2 (Variables|/Game/Characters/AI/BP_AlertLight.BP_AlertLight_C|GetSpotLight2 _alertlight))
  (|CallParentFunction)
  (Actor|Tick|SetActorTickEnabled _alertlight true)
  (Rendering|Components|Light|SetIntensity _spotlight 1e+05)
  (Rendering|Components|Light|SetIntensity _spotlight2 1e+05)
  (Utilities|FlowControl|Delay 2e+01)
  (Rendering|Components|Light|SetIntensity _spotlight 0.0)
  (Rendering|Components|Light|SetIntensity _spotlight2 0.0)
  (Actor|Tick|SetActorTickEnabled _alertlight))

(fn ConstructionScript)