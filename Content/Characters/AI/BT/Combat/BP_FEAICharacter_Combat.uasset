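; Combat AI character that fires a rifle at the player and carries an eye widget oriented to the camera.
; It caches player 0's character on BeginPlay and re-orients the eye widget every tick from camera rotation, with roll and pitch flipped.
; ShootRifle always spawns a BP_Bullet at the muzzle, aimed slightly above the player's origin along the AI's up vector.
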(event EventTick
  (params (DeltaSeconds :type Float%20%28single-precision%29))
  (bind _returnvalue (Game|GetPlayerCameraManager 0))
  (bind _eyewidget (Variables|Default|GetEyeWidget))
  (bind _returnvalue_2 (Camera|GetCameraRotation _returnvalue))
  (Utilities|IsValid _eyewidget
    (:Is%20Valid
      (Transformation|SetWorldRotation _eyewidget (Math|Rotator|MakeRotator (+ (.roll _returnvalue_2) 1.8e+02) (+ (.pitch _returnvalue_2) 1.8e+02) (.yaw _returnvalue_2)) false false))))

(event EventBeginPlay
  (Variables|Default|SetPlayerCharacter (Game|GetPlayerCharacter 0)))

(fn ConstructionScript)

(fn ShootRifle
  (bind _muzzle (Variables|Default|GetMuzzle))
  (bind _returnvalue (Transformation|GetWorldTransform _muzzle))
  (Game|SpawnActorfromClass "/Game/Characters/AI/BP_Bullet.BP_Bullet_C" (Math|Transform|MakeTransform (.location _returnvalue) (Math|Rotator|FindLookatRotation (Transformation|GetWorldLocation _muzzle) (+ (Transformation|GetActorLocation (Variables|Default|GetPlayerCharacter)) (* (Transformation|GetActorUpVector) 5e+01))) (.scale _returnvalue)) "AlwaysSpawn" 0 0))