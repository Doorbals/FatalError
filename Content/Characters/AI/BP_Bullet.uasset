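; BP_Bullet is an AI projectile actor that damages player characters on impact and removes itself after a three-second lifetime.
; On hit it spawns a green explosion emitter, then applies GE_TakeDamage through the struck FEPlayerCharacter's own Ability System Component and prints the resulting health.
; It is destroyed after damaging a player or hitting any other actor, but a player without a valid component leaves it alive until the timeout.
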(event EventBeginPlay
  (Utilities|FlowControl|Delay 3.0)
  (Actor|DestroyActor))

(event Collision|EventActorBeginOverlap
  (params (OtherActor :type Actor%20Object%20Reference)))

(event EventTick
  (params (DeltaSeconds :type Float%20%28single-precision%29)))

(event Collision|EventHit
  (params (MyComp :type Primitive%20Component%20Object%20Reference) (Other :type Actor%20Object%20Reference) (OtherComp :type Primitive%20Component%20Object%20Reference) (bSelfMoved :type Boolean) (HitLocation :type Vector :default "0, 0, 0") (HitNormal :type Vector :default "0, 0, 0") (NormalImpulse :type Vector :default "0, 0, 0") (Hit :type Hit%20Result%20Structure%20%28by%20ref%29))
  (Effects|SpawnEmitteratLocation "/Game/DownloadAssets/BeamsAndLazers/Particles/P_ExplosionGreen.P_ExplosionGreen" HitLocation)
  (bind _asfeplayer_character (Utilities|Casting|CastToFEPlayerCharacter Other)
    (:then
      (Utilities|IsValid (Ability|GetAbilitySystemComponent _asfeplayer_character)
        (:Is%20Valid
          (GameplayEffects|ApplyGameplayEffectToSelf (Ability|GetAbilitySystemComponent _asfeplayer_character) "/Game/Characters/Player/GAS/Effect/GE_TakeDamage.GE_TakeDamage_C" 0.0 (GameplayEffects|MakeEffectContext (Ability|GetAbilitySystemComponent _asfeplayer_character)))
          (bind _returnvalue (GameplayAttributes|GetAttributeSet (Ability|GetAbilitySystemComponent _asfeplayer_character) "/Script/FatalError.FEAttributeSetBase"))
          (bind _asfeattribute_set_base (Utilities|Casting|CastToFEAttributeSetBase _returnvalue))
          (Development|PrintString (Utilities|String|ToString(Float) (.currentvalue (Variables|/Script/FatalError.FEAttributeSetBase|GetHealth _asfeattribute_set_base))))
          (Actor|DestroyActor))))
    (:CastFailed
      (Actor|DestroyActor))))

(fn ConstructionScript)