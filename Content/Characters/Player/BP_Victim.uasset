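; BP_Victim is a character that can be stealth-assassinated from behind.
; StalthBackAssassinate sets mesh collision to overlap pawns, plays the being-attacked montage, flags ABP_Victim as dead and disables the AssasinatedArea collision.
; It returns the AssasinREP location and the victim's rotation to the caller, presumably to position the attacker.
; A separate Ragdoll event enables mesh physics after a short delay.
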(event Custom|Ragdoll
  (Utilities|FlowControl|Delay 2.5)
  (Physics|SetSimulatePhysics (Variables|Character|GetMesh) true))

(fn ConstructionScript)

(fn StalthBackAssassinate
  (Collision|SetCollisionResponsetoChannel (Variables|Character|GetMesh) "ECC_Pawn" "ECR_Overlap")
  (Animation|PlayAnimMontage "/Game/Characters/Player/Animation/Montages/AM_BeingAttacked.AM_BeingAttacked" 1.0 "None")
  (bind _asabp_victim (Utilities|Casting|CastToABP_Victim (Components|SkeletalMesh|GetAnimInstance (Variables|Character|GetMesh))))
  (Variables|/Game/Characters/Player/ABP_Victim.ABP_Victim_C|SetCharacterDead _asabp_victim true)
  (Collision|SetCollisionResponsetoAllChannels (Variables|Default|GetAssasinatedArea) "ECR_Ignore")
  (return (Transformation|GetWorldLocation (Variables|Default|GetAssasin%20REP)) (Transformation|GetActorRotation)))