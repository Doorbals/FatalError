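; Player character Blueprint that adds ledge jumps (left, right, back) and ledge release while climbing.
; While in one climb state, Tick computes arced launch velocities toward arrow components.
; Jump input picks a braced or hanging montage, then releases, launches and turns the character through a gated rotation.
; Direction comes from ABP_Base flags, with hop-back set by its own input; otherwise a room check can change the climb state.
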(event Custom|Start%20Rotate
  ;[0.3316 0.3316 0.3316 1 40] Rotate
  (Utilities|FlowControl|Gate true) ; enters at Open
)

(event Custom|LeftJumpTracer
  ;[1 0.3184 0.1481 1 40] Jump Tracers
  ;;[0.3316 0.3316 0.3316 1 40] Left Jump Tracer
  (if (Variables|Default|GetbCanMoveLeft)
    (Variables|Default|SetCanJumpLeft false)
    (else
      (Variables|Default|SetCanJumpLeft true)
      (bind _outlaunchvelocity (Game|SuggestProjectileVelocityCustomArc (Transformation|GetActorLocation) (Transformation|GetWorldLocation (Variables|Default|GetLeftJumpArrow)) 0.0 0.4))
      (Variables|Default|SetLeftJumpLaunchVel (Utilities|LauchVelocity _outlaunchvelocity)))))

(event Custom|JumpBackTracer
  ;[1 0.3184 0.1481 1 40] Jump Tracers
  ;;[0.3316 0.3316 0.3316 1 40] Jump Back Tracer
  (Variables|Default|SetCanJumpBack true)
  (bind _outlaunchvelocity (Game|SuggestProjectileVelocityCustomArc (Transformation|GetActorLocation) (Transformation|GetWorldLocation (Variables|Default|GetBackJumpArrow)) 0.0 0.4))
  (Variables|Default|SetJumpBackVel (Utilities|LauchVelocity _outlaunchvelocity)))

(event Custom|Set%20Rotate
  ;[0.3316 0.3316 0.3316 1 40] Rotate
  (Utilities|FlowControl|Gate true
    (:Exit
      (Transformation|SetActorRotation (Class|KismetMathLibrary|RInterptoConstant (Transformation|GetActorRotation) (Variables|Default|GetCharacter%20Rotation%20Rate) (Utilities|Time|GetWorldDeltaSeconds) 3e+02)))))

(event Custom|End%20Rotate
  ;[0.3316 0.3316 0.3316 1 40] Rotate
  (Utilities|FlowControl|Gate true) ; enters at Close
)

(event Custom|RightJumpTracer
  ;[1 0.3184 0.1481 1 40] Jump Tracers
  ;;[0.3316 0.3316 0.3316 1 40] Right Jump Tracer
  (if (Variables|Default|GetbCanMoveRight)
    (Variables|Default|SetCanJumpRight false)
    (else
      (Variables|Default|SetCanJumpRight true)
      (bind _outlaunchvelocity (Game|SuggestProjectileVelocityCustomArc (Transformation|GetActorLocation) (Transformation|GetWorldLocation (Variables|Default|GetRightJumpArrow)) 0.0 0.4))
      (Variables|Default|SetRightJumpLaunchVel (Utilities|LauchVelocity _outlaunchvelocity)))))

(event Input|EnhancedActionEvents|EnhancedInputActionIA_ReleaseLedge
  (params (ActionValue :type Boolean) (ElapsedSeconds :type Float%20%28double-precision%29) (TriggeredSeconds :type Float%20%28double-precision%29) (InputAction :type Input%20Action%20Object%20Reference :default "/Game/Characters/Input/Actions/IA_ReleaseLedge.IA_ReleaseLedge"))
  ;[0.1295 0.3002 1 1 40] Climb Input Actions
  ;;[0.3316 0.3316 0.3316 1 40] IA_ReleaseEdge
  (:Started
    (switch Utilities|FlowControl|Switch|SwitchonEFEMovementState (Variables|Default|GetMovementState)
      (:Climb
        (if (Utilities|Enum|Equal(Enum) (Variables|/Game/Characters/Player/ClimbingSystem/ClimbingComponent.ClimbingComponent_C|GetClimbState (Variables|Default|GetClimbingComponent)) "NewEnumerator2")
          (Default|ReleaseLedge (Variables|Default|GetClimbingComponent) "NewEnumerator0"))))))

(event Input|EnhancedActionEvents|EnhancedInputActionIA_HopBack
  (params (ActionValue :type Boolean) (ElapsedSeconds :type Float%20%28double-precision%29) (TriggeredSeconds :type Float%20%28double-precision%29) (InputAction :type Input%20Action%20Object%20Reference :default "/Game/Characters/Input/Actions/IA_HopBack.IA_HopBack"))
  ;[0.1295 0.3002 1 1 40] Climb Input Actions
  ;;[0.3316 0.3316 0.3316 1 40] IA_HopBack
  (:Triggered
    (bind _asabp_base (Utilities|Casting|CastToABP_Base (Components|SkeletalMesh|GetAnimInstance (Variables|Character|GetMesh))))
    (if (Utilities|Enum|Equal(Enum) (Variables|/Game/Characters/Player/ClimbingSystem/ClimbingComponent.ClimbingComponent_C|GetClimbState (Variables|Default|GetClimbingComponent)) "NewEnumerator2")
      (Variables|/Game/Characters/Player/Animation/ABP_Base.ABP_Base_C|SetIsHopBack _asabp_base true)
      (else
        (Variables|/Game/Characters/Player/Animation/ABP_Base.ABP_Base_C|SetIsHopBack _asabp_base false :!label _label))))
  (:Canceled
    (goto _label))
  (:Completed
    (goto _label)))

(event Input|EnhancedActionEvents|EnhancedInputActionIA_Jump
  (params (ActionValue :type Boolean) (ElapsedSeconds :type Float%20%28double-precision%29) (TriggeredSeconds :type Float%20%28double-precision%29) (InputAction :type Input%20Action%20Object%20Reference :default "/Game/Characters/Input/Actions/IA_Jump.IA_Jump"))
  (bind _returnvalue (Transformation|GetActorRotation))
  (bind _climbingcomponent (Variables|Default|GetClimbingComponent))
  (bind _climbingcomponent_2 (Variables|Default|GetClimbingComponent))
  (bind _climbingcomponent_3 (Variables|Default|GetClimbingComponent))
  (bind _fullhang (Variables|/Game/Characters/Player/ClimbingSystem/ClimbingComponent.ClimbingComponent_C|GetFullHang _climbingcomponent_2))
  ;[0.1295 0.3002 1 1 40] Climb Input Actions
  ;;[0.3316 0.3316 0.3316 1 40] IA_Jump
  (:Triggered
    (switch Utilities|FlowControl|Switch|SwitchonEFEMovementState (Variables|Default|GetMovementState)
      (:Climb
        (if (Utilities|Enum|Equal(Enum) (Variables|/Game/Characters/Player/ClimbingSystem/ClimbingComponent.ClimbingComponent_C|GetClimbState (Variables|Default|GetClimbingComponent)) "NewEnumerator2")
          (bind _asabp_base (Utilities|Casting|CastToABP_Base (Components|SkeletalMesh|GetAnimInstance (Variables|Character|GetMesh))))
          (if (Variables|/Game/Characters/Player/Animation/ABP_Base.ABP_Base_C|GetIsHopBack _asabp_base)
            (if _fullhang
              (Variables|Default|SetJumpAnim "/Game/Characters/Player/Animation/Montages/AM_FullJumpBack.AM_FullJumpBack")
              (else
                (Variables|Default|SetJumpAnim "/Game/Characters/Player/Animation/Montages/AM_BracedJumpBack.AM_BracedJumpBack")))
            (Variables|Default|SetCharacterRotationZ 179.0)
            (Variables|Default|SetJumpVel (Variables|Default|GetJumpBackVel))
            (Variables|Default|SetbMovementEnabled false :!label _label)
            (Animation|Montage|PlayMontage (Variables|Character|GetMesh) (Variables|Default|GetJumpAnim) 0.8
              (:then
                (Utilities|FlowControl|Delay 0.35)
                (Default|ReleaseLedge _climbingcomponent "NewEnumerator0")
                (Variables|/Game/Characters/Player/ClimbingSystem/ClimbingComponent.ClimbingComponent_C|SetClimbState _climbingcomponent "NewEnumerator5")
                (Character|LaunchCharacter (Variables|Default|GetJumpVel) true true)
                (CallFunction|StartRotate)
                (Variables|Default|SetCharacter%20Rotation%20Rate (Math|Rotator|MakeRotator (.roll _returnvalue) (.pitch _returnvalue) (+ (.yaw _returnvalue) (Variables|Default|GetCharacterRotationZ))))
                (Utilities|FlowControl|Delay 0.8)
                (CallFunction|EndRotate)
                (bind _asabp_base_2 (Utilities|Casting|CastToABP_Base (Components|SkeletalMesh|GetAnimInstance (Variables|Character|GetMesh))))
                (Variables|/Game/Characters/Player/Animation/ABP_Base.ABP_Base_C|SetIsHopBack _asabp_base_2 false)))
            (elif (and (not (Variables|/Game/Characters/Player/Animation/ABP_Base.ABP_Base_C|GetCanMoveLeft _asabp_base)) (Variables|/Game/Characters/Player/Animation/ABP_Base.ABP_Base_C|GetMoving%20Left _asabp_base))
              (if _fullhang
                (Variables|Default|SetJumpAnim "/Game/Characters/Player/Animation/Montages/AM_FullJumpLeft.AM_FullJumpLeft")
                (else
                  (Variables|Default|SetJumpAnim "/Game/Characters/Player/Animation/Montages/AM_BracedJumpLeft.AM_BracedJumpLeft")))
              (Variables|Default|SetCharacterRotationZ -9e+01)
              (Variables|Default|SetJumpVel (Variables|Default|GetLeftJumpLaunchVel))
              (goto _label)
              (elif (and (not (Variables|/Game/Characters/Player/Animation/ABP_Base.ABP_Base_C|GetCanMoveRight _asabp_base)) (Variables|/Game/Characters/Player/Animation/ABP_Base.ABP_Base_C|GetMoving%20Right _asabp_base))
                (if _fullhang
                  (Variables|Default|SetJumpAnim "/Game/Characters/Player/Animation/Montages/AM_FullJumpRight.AM_FullJumpRight")
                  (else
                    (Variables|Default|SetJumpAnim "/Game/Characters/Player/Animation/Montages/AM_BracedJumpRight.AM_BracedJumpRight")))
                (Variables|Default|SetCharacterRotationZ 9e+01)
                (Variables|Default|SetJumpVel (Variables|Default|GetRightJumpLaunchVel))
                (goto _label)
                (else
                  (bind _canstand (Default|RoomCheck _climbingcomponent_3))
                  (if _canstand
                    (Variables|/Game/Characters/Player/ClimbingSystem/ClimbingComponent.ClimbingComponent_C|SetClimbState _climbingcomponent_3 "NewEnumerator3")))))))))))

(event EventTick
  (params (DeltaSeconds :type Float%20%28single-precision%29))
  ;[0.3316 0.3316 0.3316 1 40] Tick
  (if (AI|Components|NavMovement|IsFalling (Variables|Character|GetCharacterMovement))
    (CallFunction|SetRotate))
  (if (Utilities|Enum|Equal(Enum) (Variables|/Game/Characters/Player/ClimbingSystem/ClimbingComponent.ClimbingComponent_C|GetClimbState (Variables|Default|GetClimbingComponent)) "NewEnumerator2")
    (Utilities|FlowControl|Sequence
      (:then_0
        (if (and (< (Variables|Default|GetMovingLeftRight) 0.0) (not (Variables|Default|GetbCanMoveLeft)))
          (CallFunction|LeftJumpTracer)
          (else
            (Variables|Default|SetCanJumpLeft false))))
      (:then_1
        (if (and (> (Variables|Default|GetMovingLeftRight) 0.0) (not (Variables|Default|GetbCanMoveRight)))
          (CallFunction|RightJumpTracer)
          (else
            (Variables|Default|SetCanJumpRight false))))
      (:then_2
        (CallFunction|JumpBackTracer)))))

(fn ConstructionScript)