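; Gameplay ability that lets the player character assassinate a nearby target.
; On activation it gathers overlapping actors implementing the FEI_Assassination interface and cancels if none are found.
; Otherwise it calls AssassinatedMessage on the first one, then plays the assassinate montage with a "Victim" motion warp target set to the returned location and rotation.
; The ability ends and clears the candidate list when the montage completes, blends out or is interrupted.
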(event Ability|EventActivateAbility
  (bind _returnvalue (Ability|GetActorInfo))
  (bind _implementedactors (Variables|Default|GetImplementedActors))
  (bind _asbp_feplayer_character (Utilities|Casting|CastToBP_FEPlayerCharacter (.avataractor _returnvalue)))
  (for _array_element (Collision|GetOverlappingActors (.avataractor _returnvalue) 0 :!class /Script/Engine.Actor)
    (if (Utilities|DoesObjectImplementInterface _array_element "/Script/FatalError.FEI_Assassination")
      (Utilities|Array|Add (Variables|Default|GetImplementedActors) _array_element)))
  (if (> (Utilities|Array|Length _implementedactors) 0)
    (bind (_location _rotation) (Class|FEIAssassination|Assassinated(Message) (Utilities|Array|Get(acopy) _implementedactors)))
    (|PlayMontageandWaitProxy "None" "/Game/Characters/Player/Animation/Montages/AM_Assassinate.AM_Assassinate" 1.0 "None" true 1.0 0.0
      (:then
        (Class|MotionWarpingComponent|AddorUpdateWarpTarget (Variables|/Game/Characters/Player/BP_FEPlayerCharacter.BP_FEPlayerCharacter_C|GetMotionWarping _asbp_feplayer_character) (Utilities|Struct|MakeMotionWarpingTarget "Victim" _location _rotation 0 "None" false)))
      (:OnCompleted
        (Ability|EndAbility :!label _label)
        (Utilities|Array|Clear (Variables|Default|GetImplementedActors)))
      (:OnBlendOut
        (goto _label))
      (:OnInterrupted
        (goto _label))
      (:OnCancelled
        (goto _label)))
    (else
      (Ability|CancelAbility)
      (Utilities|Array|Clear (Variables|Default|GetImplementedActors)))))

(event Ability|EventOnEndAbility
  (params (bWasCancelled :type Boolean)))